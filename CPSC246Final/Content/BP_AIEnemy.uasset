(event `self.ReceiveBeginPlay`
  (set `self.isSeeingPlayer` false)
  (`KismetSystemLibrary.Delay` 10.0)
  (`self.RandomRoam`)
  (`GameplayStatics.SpawnSoundAttached` "/Game/SoundEffects/MonsterSteps.MonsterSteps" (`self.Mesh`) "None" (0.0 0.0 0.0) (struct) "KeepRelativeOffset" false 0.2 1.0 0.0 "/Game/SoundEffects/SA_MonsterSteps.SA_MonsterSteps" null false))

(event `self.ReceiveTick`
  (params (DeltaSeconds :type "Float (single-precision)")))

(event `self.PawnSensing.OnSeePawn`
  (params (Pawn :type "Pawn Object Reference"))
  (`|ExecutionSequence`
    (:`then_0`
      (`KismetSystemLibrary.PrintString` "SPEED SET TO 450")
      (set `CharacterMovementComponent.MaxWalkSpeed` 500.0 (`self.CharacterMovement`))
      (`|AIMoveTo` null (0.0 0.0 0.0) Pawn
        (:`then`
          (if (not (`self.isSoundPlaying?`))
            (set `self.isSoundPlaying?` true)
            (`GameplayStatics.PlaySoundAtLocation` "/Game/SoundEffects/Insidious-Scary-Violins-Sound-Effect.Insidious-Scary-Violins-Sound-Effect" (`self.K2_GetActorLocation` Pawn) (struct) 0.05 1.0 0.0 null null null)
            (`KismetSystemLibrary.Delay` 7.0)
            (set `self.isSoundPlaying?` false)))))
    (:`then_1`
      (`KismetSystemLibrary.RetriggerableDelay` 1.0)
      (`self.RandomRoam`))))

(event `RandomRoam`
  (`KismetSystemLibrary.PrintString` "SPEED SET TO 250")
  (set `CharacterMovementComponent.MaxWalkSpeed` 250.0 (`self.CharacterMovement`))
  (`|AIMoveTo` self (0.0 0.0 0.0) (`GameplayStatics.GetPlayerCharacter` 0)))

(event `self.Box.OnComponentBeginOverlap`
  (params (OverlappedComponent :type "PrimitiveComponent Object Reference") (OtherActor :type "Actor Object Reference") (OtherComp :type "PrimitiveComponent Object Reference") (OtherBodyIndex :type Integer) (bFromSweep :type Boolean) (SweepResult :type "HitResult Structure (by ref)"))
  (cast `/Game/FirstPersonBP/Blueprints/FirstPersonCharacter` OtherActor)
  (bind _returnvalue (`|CreateWidget` "/Game/YouLost.YouLost_C"))
  (`UserWidget.AddToViewport` _returnvalue 0)
  (`GameplayStatics.SetGamePaused` true))

(fn `UserConstructionScript`)